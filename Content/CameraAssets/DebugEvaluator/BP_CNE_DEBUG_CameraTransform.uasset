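; BP_CNE_DEBUG_CameraTransform is a Blueprint camera node evaluator for debugging the camera transform.
; On each camera node tick it can print the location and rotation from the camera data's pose as labelled strings.
; Both prints sit behind a branch hard-coded to false, so the node currently outputs nothing.
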(event `self.TickCameraNode`
  (params (DeltaTime :type "Float (single-precision)"))
  (bind (_returnvalue_location _returnvalue_rotation) (break `BlueprintCameraPose` (`BlueprintCameraEvaluationDataFunctionLibrary.GetCameraPose` (`self.CameraData`))))
  (if false
    (`KismetSystemLibrary.PrintString` (`KismetStringLibrary.Concat_StrStr` "Camera Location : " (`KismetStringLibrary.Conv_VectorToString` _returnvalue_location)))
    (`KismetSystemLibrary.PrintString` (`KismetStringLibrary.Concat_StrStr` "Camera Rotation: " (`KismetStringLibrary.Conv_RotatorToString` _returnvalue_rotation)))))