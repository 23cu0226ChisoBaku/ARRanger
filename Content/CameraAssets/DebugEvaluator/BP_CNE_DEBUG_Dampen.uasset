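; BP_CNE_DEBUG_Dampen is a debug camera node evaluator for inspecting camera dampening values.
; On each camera node tick, it is set up to read two float camera variables from the camera data and print them as labeled forward and horizontal dampen strings.
; The whole read-and-print chain sits behind a constant false branch, so the node currently outputs nothing.
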(event `self.TickCameraNode`
  (params (DeltaTime :type "Float (single-precision)"))
  (bind _cameradata (`self.CameraData`))
  (if false
    (bind _returnvalue (`BlueprintCameraVariableTableFunctionLibrary.GetFloatCameraVariable` _cameradata "/Game/CameraAssets/CVC_ARRangerCharacter.CVC_ARRangerCharacter.FloatCameraVariable_1"))
    (`KismetSystemLibrary.PrintString` (`KismetStringLibrary.Concat_StrStr` "Forward Dampen :" (`KismetStringLibrary.Conv_DoubleToString` _returnvalue)))
    (bind _returnvalue_2 (`BlueprintCameraVariableTableFunctionLibrary.GetFloatCameraVariable` _cameradata "/Game/CameraAssets/CVC_ARRangerCharacter.CVC_ARRangerCharacter.FloatCameraVariable_2"))
    (`KismetSystemLibrary.PrintString` (`KismetStringLibrary.Concat_StrStr` "Horizontal Dampen :" (`KismetStringLibrary.Conv_DoubleToString` _returnvalue_2)))))