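; Camera node Blueprint, named as a fallback idle camera offset for the ARRanger character, that currently only prints "Walk" or "Run" each tick and applies no offset.
; Walk and run are classified by comparing the pawn's squared XY last input against dead-zone and run thresholds, gated by horizontal velocity and a ground check.
; IsOnGround returns IsFalling un-negated, so both states register only while the pawn is falling.
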(event `self.TickCameraNode`
  (params (DeltaTime :type "Float (single-precision)"))
  (if (`KismetSystemLibrary.IsValid` (`self.GetPlayerController`))
    (if (`self.IsMoving_Walk`)
      (`KismetSystemLibrary.PrintString` "Walk")
      (elif (`self.IsMoving_Run`)
        (`KismetSystemLibrary.PrintString` "Run")))))

(fn `HasOnGroundMovementVelocity`
  (returns (Result :type Boolean))
  (bind _returnvalue (`self.GetPlayerController`))
  (return (and (`KismetSystemLibrary.IsValid` _returnvalue) (>= (`KismetMathLibrary.VSizeXY` (`NavMovementInterface.GetVelocityForNavMovement` (`Pawn.GetMovementComponent` (`Controller.K2_GetPawn` _returnvalue)))) (`self.MoveVelocityLengthThreshold`)) (`self.IsOnGround`))))

(fn `IsMoving_Run`
  (returns (Result :type Boolean))
  (bind _returnvalue (`self.GetPlayerController`))
  (return (and (`KismetSystemLibrary.IsValid` _returnvalue) (and (`self.HasOnGroundMovementVelocity`) (>= (`KismetMathLibrary.VSizeXYSquared` (`PawnMovementComponent.GetLastInputVector` (`Pawn.GetMovementComponent` (`Controller.K2_GetPawn` _returnvalue)))) (`KismetMathLibrary.Square` (`KismetMathLibrary.FMax` (`self.MinRunInputValue_Temp`) (`self.DeadZone_Temp`))))))))

(fn `IsMoving_Walk`
  (returns (Result :type Boolean))
  (bind _returnvalue (`self.GetPlayerController`))
  (bind _returnvalue_2 (`KismetMathLibrary.VSizeXYSquared` (`PawnMovementComponent.GetLastInputVector` (`Pawn.GetMovementComponent` (`Controller.K2_GetPawn` _returnvalue)))))
  (return (and (`KismetSystemLibrary.IsValid` _returnvalue) (and (`self.HasOnGroundMovementVelocity`) (and (>= _returnvalue_2 (`KismetMathLibrary.Square` (`self.DeadZone_Temp`))) (< _returnvalue_2 (`KismetMathLibrary.Square` (`KismetMathLibrary.FMax` (`self.MinRunInputValue_Temp`) (`self.DeadZone_Temp`)))))))))

(fn `IsOnGround`
  (returns (Result :type Boolean))
  (bind _returnvalue (`self.GetPlayerController`))
  (return (and (`KismetSystemLibrary.IsValid` _returnvalue) (`NavMovementInterface.IsFalling` (`Pawn.GetMovementComponent` (`Controller.K2_GetPawn` _returnvalue))))))