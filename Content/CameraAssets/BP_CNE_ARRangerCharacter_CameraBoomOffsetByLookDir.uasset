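; Gameplay Cameras node evaluator for the AR Ranger character that adjusts the camera boom offset by look pitch.
; Each tick it reads the player camera's pitch, building a 0-to-1 weight as the view tilts down to -45 degrees.
; The weight scales a clamped X offset plus an extra distance split into back and up by cosine and sine, written to a vector camera variable.
; A boolean variable flags pitch above -30 degrees.
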(event `self.TickCameraNode`
  (params (DeltaTime :type "Float (single-precision)"))
  (bind _pitch (.pitch (`PlayerCameraManager.GetCameraRotation` (`PlayerController.PlayerCameraManager` (`self.GetPlayerController`)))))
  (bind _returnvalue (`KismetMathLibrary.Abs` _pitch))
  (bind _returnvalue_2 (`KismetMathLibrary.FClamp` (/ _pitch -45.0)))
  (bind _returnvalue_3 (* _returnvalue_2 (`self.ExtraOffset`)))
  (if (`KismetSystemLibrary.IsValid` (`self.GetPlayerController`))
    (`BlueprintCameraVariableTableFunctionLibrary.SetBooleanCameraVariable` (`self.CameraData`) "/Game/CameraAssets/CVC_ARRangerCharacter.CVC_ARRangerCharacter.BooleanCameraVariable_0" (> _pitch -30.0))
    (`BlueprintCameraVariableTableFunctionLibrary.SetVector3CameraVariable` (`self.CameraData`) "/Game/CameraAssets/CVC_ARRangerCharacter.CVC_ARRangerCharacter.Vector3dCameraVariable_2" (`KismetMathLibrary.MakeVector` (- (`KismetMathLibrary.FClamp` (* (`self.BoomArmXOffset`) _returnvalue_2) (`self.BoomArmXOffset`) 0.0) (* (`KismetMathLibrary.DegCos` _returnvalue) _returnvalue_3)) 0.0 (* _returnvalue_3 (`KismetMathLibrary.DegSin` _returnvalue))))))