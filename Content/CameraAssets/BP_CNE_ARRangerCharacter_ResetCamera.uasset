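; A Gameplay Cameras Blueprint node evaluator that ends a camera reset for the ranger character.
; On each node tick it finds the owning BP_ThirdPersonCharacter and derives its facing as a look-at rotation along its forward vector.
; When the camera pose rotation matches that facing within a tiny tolerance, it switches the character's camera rig back to Default.
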(event `self.TickCameraNode`
  (params (DeltaTime :type "Float (single-precision)"))
  (bind _returnvalue (`self.FindEvaluationContextOwnerActor` "/Game/ThirdPerson/Blueprints/BP_ThirdPersonCharacter.BP_ThirdPersonCharacter_C"))
  (bind (_returnvalue_location _returnvalue_rotation) (break `BlueprintCameraPose` (`BlueprintCameraEvaluationDataFunctionLibrary.GetCameraPose` (`self.CameraData`))))
  (bind _returnvalue_2 (`Actor.K2_GetActorLocation` _returnvalue))
  (if (`KismetSystemLibrary.IsValid` _returnvalue)
    (if (== (`KismetMathLibrary.FindLookAtRotation` _returnvalue_2 (+ (`Actor.GetActorForwardVector` _returnvalue) _returnvalue_2)) _returnvalue_rotation :`ErrorTolerance` 1e-05)
      (`ARRangerCharacter.SetCameraRig` _returnvalue "Default"))))