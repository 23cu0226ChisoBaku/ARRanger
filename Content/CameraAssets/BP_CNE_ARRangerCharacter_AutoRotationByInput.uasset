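; Camera node for the AR Ranger character that decides when input-based auto-rotation Step 1 is active, via a boolean camera variable.
; Each tick it compares pawn planar speed to a threshold and clears the flag below it.
; Above it, velocity direction is dotted with camera forward flattened against the actor's up vector, setting the flag within the SwitchToStep2Deg angle.
; Outside that angle the flag is left unchanged.
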(event `self.TickCameraNode`
  (params (DeltaTime :type "Float (single-precision)"))
  (bind _returnvalue (`self.GetPlayerController`))
  (bind _returnvalue_2 (`Controller.K2_GetPawn` _returnvalue))
  (bind _returnvalue_3 (`Actor.GetActorUpVector` _returnvalue_2))
  (bind _returnvalue_4 (`KismetMathLibrary.GetForwardVector` (`PlayerCameraManager.GetCameraRotation` (`PlayerController.PlayerCameraManager` _returnvalue))))
  (bind _returnvalue_5 (`NavMovementComponent.GetVelocityForNavMovement` (`Pawn.GetMovementComponent` _returnvalue_2)))
  (if (`KismetSystemLibrary.IsValid` _returnvalue)
    (if (>= (`KismetMathLibrary.VSizeXY` _returnvalue_5) (`self.EnableAutoRotateSpeedThreshold`))
      (if (>= (`KismetMathLibrary.Dot_VectorVector` (`KismetMathLibrary.Normal` _returnvalue_5) (`KismetMathLibrary.Vector_NormalUnsafe` (- _returnvalue_4 (* (`KismetMathLibrary.Dot_VectorVector` _returnvalue_4 _returnvalue_3) _returnvalue_3)))) (`KismetMathLibrary.DegCos` (`self.SwitchToStep2Deg`)))
        (`BlueprintCameraVariableTableFunctionLibrary.SetBooleanCameraVariable` (`self.CameraData`) "/Game/CameraAssets/CVC_ARRangerCharacter.CVC_ARRangerCharacter.BooleanCameraVariable_1" true) ; Enable Step1
      )
      (else
        (`BlueprintCameraVariableTableFunctionLibrary.SetBooleanCameraVariable` (`self.CameraData`) "/Game/CameraAssets/CVC_ARRangerCharacter.CVC_ARRangerCharacter.BooleanCameraVariable_1")))))