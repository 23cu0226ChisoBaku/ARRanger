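; Blueprint camera node for the AR Ranger character that dampens camera motion during jumps.
; Each tick, while the controlled pawn is falling, it writes a Z-only offset to a vector camera variable, otherwise it writes zero.
; The offset is the cosine of scaled vertical velocity times MaxZOffset, clamped between MaxZOffset and zero, so it peaks near the jump apex.
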(event `self.TickCameraNode`
  (params (DeltaTime :type "Float (single-precision)"))
  (bind _returnvalue (`self.GetPlayerController`))
  (bind _maxzoffset (`self.MaxZOffset`))
  (bind _returnvalue_2 (`Pawn.GetMovementComponent` (`Controller.K2_GetPawn` _returnvalue)))
  (if (`KismetSystemLibrary.IsValid` _returnvalue)
    (if (`NavMovementComponent.IsFalling` _returnvalue_2)
      (`BlueprintCameraVariableTableFunctionLibrary.SetVector3CameraVariable` (`self.CameraData`) "/Game/CameraAssets/CVC_ARRangerCharacter.CVC_ARRangerCharacter.Vector3dCameraVariable_3" (`KismetMathLibrary.MakeVector` 0.0 0.0 (`KismetMathLibrary.FClamp` (* (`KismetMathLibrary.Cos` (* (.z (`NavMovementInterface.GetVelocityForNavMovement` _returnvalue_2)) (`self.CoefficientOfCos`))) _maxzoffset) _maxzoffset 0.0)))
      (else
        (`BlueprintCameraVariableTableFunctionLibrary.SetVector3CameraVariable` (`self.CameraData`) "/Game/CameraAssets/CVC_ARRangerCharacter.CVC_ARRangerCharacter.Vector3dCameraVariable_3" (`KismetMathLibrary.MakeVector` 0.0))))))