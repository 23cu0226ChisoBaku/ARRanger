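; Gameplay camera node for the AR Ranger character that adjusts damping and forward offset as the player moves.
; Above a speed threshold with pitch below a limit, facing toward the camera raises damping by the dot product of flattened camera and pawn forwards.
; It also eases in a pitch-corrected offset through a timed curve, written to camera variables.
; Slowing eases the offset out; exceeding the pitch limit zeroes damping.
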(event `self.TickCameraNode`
  (params (DeltaTime :type "Float (single-precision)"))
  (bind _returnvalue (`self.GetPlayerController`))
  (bind _forwardoffsettimeinterval (`self.ForwardOffsetTimeInterval`))
  (bind _forwardoffsettimeinterval_2 (`self.ForwardOffsetTimeInterval`))
  (bind _cameradata (`self.CameraData`))
  (bind _cameradata_2 (`self.CameraData`))
  (bind _returnvalue_2 (`Controller.K2_GetPawn` _returnvalue))
  (bind _returnvalue_3 (`Actor.GetActorUpVector` _returnvalue_2))
  (bind _returnvalue_4 (`KismetMathLibrary.FClamp` (- (`self.ForwardOffsetTimeCnt`) DeltaTime) 0.0 _forwardoffsettimeinterval))
  (bind _returnvalue_5 (`PlayerCameraManager.GetCameraRotation` (`PlayerController.PlayerCameraManager` _returnvalue)))
  (bind _pitch (.pitch _returnvalue_5))
  (bind _returnvalue_6 (`KismetMathLibrary.GetForwardVector` _returnvalue_5))
  (bind _returnvalue_7 (`KismetMathLibrary.Abs` _pitch))
  (bind _returnvalue_8 (`KismetMathLibrary.Dot_VectorVector` (`KismetMathLibrary.Vector_NormalUnsafe` (- _returnvalue_6 (* (`KismetMathLibrary.Dot_VectorVector` _returnvalue_6 _returnvalue_3) _returnvalue_3))) (`Actor.GetActorForwardVector` _returnvalue_2)))
  (if (`KismetSystemLibrary.IsValid` _returnvalue)
    (if (>= (`KismetMathLibrary.VSizeXY` (`NavMovementInterface.GetVelocityForNavMovement` (`Pawn.GetMovementComponent` _returnvalue_2))) 150.0)
      (if (< _pitch 15.0)
        (if (< _returnvalue_8 0.0)
          (bind _returnvalue_9 (`BlueprintCameraVariableTableFunctionLibrary.GetFloatCameraVariable` _cameradata_2 "/Game/CameraAssets/CVC_ARRangerCharacter.CVC_ARRangerCharacter.FloatCameraVariable_3"))
          (`BlueprintCameraVariableTableFunctionLibrary.SetFloatCameraVariable` _cameradata_2 "/Game/CameraAssets/CVC_ARRangerCharacter.CVC_ARRangerCharacter.FloatCameraVariable_1" (+ _returnvalue_9 (`KismetMathLibrary.Abs` (* _returnvalue_8 (`self.ForwardDampen`)))))
          (bind _output_get (set `self.ForwardOffsetTimeCnt` (`KismetMathLibrary.FClamp` (+ DeltaTime (`self.ForwardOffsetTimeCnt`)) 0.0 _forwardoffsettimeinterval_2)))
          (bind _output_get_2 (set `self.PreviousForwardOffsetVector` (`KismetMathLibrary.MakeVector` (* _returnvalue_8 (* (`self.ForwardOffset`) (`KismetMathLibrary.DegCos` _returnvalue_7))) 0.0 (* _returnvalue_8 (* (`KismetMathLibrary.DegSin` _returnvalue_7) (`self.ForwardOffset`))))))
          (`BlueprintCameraVariableTableFunctionLibrary.SetVector3CameraVariable` (`self.CameraData`) "/Game/CameraAssets/CVC_ARRangerCharacter.CVC_ARRangerCharacter.Vector3dCameraVariable_4" (`KismetMathLibrary.VLerp` (`KismetMathLibrary.MakeVector` 0.0) _output_get_2 (`CurveFloat.GetFloatValue` (`self.Curve_ForwardOffsetLerp`) (/ _output_get _forwardoffsettimeinterval_2))))
          (else
            (set `self.ForwardOffsetTimeCnt` 0.0)
            (bind _returnvalue_10 (`BlueprintCameraVariableTableFunctionLibrary.GetFloatCameraVariable` _cameradata "/Game/CameraAssets/CVC_ARRangerCharacter.CVC_ARRangerCharacter.FloatCameraVariable_3"))
            (`BlueprintCameraVariableTableFunctionLibrary.SetFloatCameraVariable` _cameradata "/Game/CameraAssets/CVC_ARRangerCharacter.CVC_ARRangerCharacter.FloatCameraVariable_1" _returnvalue_10)))
        (else
          (`BlueprintCameraVariableTableFunctionLibrary.SetFloatCameraVariable` (`self.CameraData`) "/Game/CameraAssets/CVC_ARRangerCharacter.CVC_ARRangerCharacter.FloatCameraVariable_1")))
      (else
        (set `self.ForwardOffsetTimeCnt` _returnvalue_4)
        (`BlueprintCameraVariableTableFunctionLibrary.SetVector3CameraVariable` (`self.CameraData`) "/Game/CameraAssets/CVC_ARRangerCharacter.CVC_ARRangerCharacter.Vector3dCameraVariable_4" (`KismetMathLibrary.VLerp` (`KismetMathLibrary.MakeVector` 0.0) (`self.PreviousForwardOffsetVector`) (`CurveFloat.GetFloatValue` (`self.Curve_ForwardOffsetLerp`) (/ _returnvalue_4 _forwardoffsettimeinterval))))))))