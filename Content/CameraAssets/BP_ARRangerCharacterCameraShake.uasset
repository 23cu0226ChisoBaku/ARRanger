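; Camera node Blueprint for the ARRanger character camera that produces a randomized positional shake offset.
; Each tick advances a timer; when the interval elapses, it takes the old target as start, picks a new target and re-rolls the interval from a range.
; Targets are random points on a sphere, limited to non-positive X and non-negative Z.
; A curve-eased lerp between them is written to a vector camera variable.
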(event `self.TickCameraNode`
  (params (DeltaTime :type "Float (single-precision)"))
  (bind (_shakecameratimeintervalrange_lowerbound _shakecameratimeintervalrange_upperbound) (break `FloatRange` (`self.ShakeCameraTimeIntervalRange`)))
  (if (>= (`self.ShakeCameraTimeCnt`) (`self.RealShakeCameraTimeInterval`))
    (set `self.StartPosition` (`self.TargetPosition`))
    (set `self.TargetPosition` (`self.GetPositionOnSphere` (`self.ShakeSphereRadius`)))
    (set `self.ShakeCameraTimeCnt` 0.0)
    (set `self.RealShakeCameraTimeInterval` (`KismetMathLibrary.RandomFloatInRange` (`.Value` (break `FloatRangeBound` _shakecameratimeintervalrange_lowerbound)) (`.Value` (break `FloatRangeBound` _shakecameratimeintervalrange_upperbound))))
    (else
      (set `self.ShakeCameraTimeCnt` (+ DeltaTime (`self.ShakeCameraTimeCnt`)))))
  (`BlueprintCameraVariableTableFunctionLibrary.SetVector3CameraVariable` (`self.CameraData`) "/Game/CameraAssets/CVC_ARRangerCharacter.CVC_ARRangerCharacter.Vector3dCameraVariable_0" (`self.CalcCameraOffset`)))

(fn `CalcCameraOffset`
  (returns (ResultPosition :type "Vector Structure"))
  (return (`KismetMathLibrary.VLerp` (`self.StartPosition`) (`self.TargetPosition`) (`CurveFloat.GetFloatValue` (`self.ShakeCurve`) (/ (`self.ShakeCameraTimeCnt`) (`self.RealShakeCameraTimeInterval`))))))

(fn `GetPositionOnSphere`
  (params (SphereRadius :type "Float (double-precision)"))
  (returns (ResultPosition :type "Vector Structure"))
  (bind _returnvalue (`KismetMathLibrary.RandomFloatInRange` (* SphereRadius -1.0)))
  (bind _returnvalue_2 (`KismetMathLibrary.MultiplyMultiply_FloatFloat` _returnvalue 2.0))
  (bind _returnvalue_3 (- (`KismetMathLibrary.MultiplyMultiply_FloatFloat` SphereRadius 2.0) _returnvalue_2))
  (bind _returnvalue_4 (`KismetMathLibrary.RandomFloatInRange` (* _returnvalue_3 -1.0) _returnvalue_3))
  (bind _returnvalue_5 (`KismetMathLibrary.Abs` _returnvalue_4))
  (return (`KismetMathLibrary.MakeVector` _returnvalue (* (`KismetMathLibrary.Sqrt` _returnvalue_5) (`KismetMathLibrary.SignOfFloat` _returnvalue_4)) (`KismetMathLibrary.Sqrt` (- (- (`KismetMathLibrary.MultiplyMultiply_FloatFloat` SphereRadius 2.0) _returnvalue_2) _returnvalue_5)))))