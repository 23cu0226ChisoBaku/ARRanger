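; BP_CNE_ARRangerCharacter_IdleStateCameraOffsets is an unfinished camera node for the ARRanger character, named for idle-state camera offsets.
; Each tick it calls ApplyYOffset, which only checks the player controller's validity and applies no offset yet.
; It then casts the controlled pawn's movement component to CharacterMovementComponent and prints horizontal navigation-movement speed as debug output.
; IsMove_Walk and one other function are empty stubs.
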(event `self.TickCameraNode`
  (params (DeltaTime :type "Float (single-precision)"))
  (bind _returnvalue (`Pawn.GetMovementComponent` (`Controller.K2_GetPawn` (`self.GetPlayerController`))))
  (`self.ApplyYOffset` DeltaTime)
  (bind `_asキャラクター移動コンポーネント` (cast `CharacterMovementComponent` _returnvalue))
  (`KismetSystemLibrary.PrintString` (`KismetStringLibrary.Conv_DoubleToString` (`KismetMathLibrary.VSizeXY` (`NavMovementInterface.GetVelocityForNavMovement` _returnvalue)))))

(fn `ApplyYOffset`
  (params (DeltaTime :type "Float (double-precision)"))
  (locals (ApplyYOffsetTimeInterval :type "Float (double-precision)"))
  (if (`KismetSystemLibrary.IsValid` (`self.GetPlayerController`))
    _))

(fn `IsMove_Walk`)

(fn `新規関数_0`)