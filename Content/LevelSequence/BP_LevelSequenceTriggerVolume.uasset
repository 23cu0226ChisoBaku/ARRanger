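; Trigger volume that plays a target Level Sequence when a player-controlled pawn overlaps it.
; It can fade out through a WBP_Fade widget and timed delay before playback, then binds to the sequence's finish event.
; On finish it can fade back in, collect garbage after that fade, and optionally destroy itself.
; Event dispatchers announce the start and end of each fade and of playback.
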(event `self.ReceiveActorBeginOverlap`
  (params (OtherActor :type "Actor Object Reference"))
  (bind _sequenceplayer (`LevelSequenceActor.SequencePlayer` (`self.TargetLevelSequencePlayer`)))
  (bind `_asポーン` (cast `Pawn` OtherActor))
  (bind `_asプレイヤーコントローラー` (cast `PlayerController` (`Pawn.GetController` `_asポーン`)))
  (if (`self.EnableFadeOut`)
    (`self.OnFadeOutStarted`)
    (bind _createdwidget (`self.FadeOut_Implementation` `_asプレイヤーコントローラー`))
    (`KismetSystemLibrary.Delay` (`self.FadeOutTime`))
    (`self.OnFadeOutEnded`)
    (`Widget.RemoveFromParent` _createdwidget))
  (if (`KismetSystemLibrary.IsValid` (`self.TargetLevelSequencePlayer`))
    (`self.OnLevelSequencePlayStarted`)
    (`MovieSceneSequencePlayer.Play` _sequenceplayer)
    (add `MovieSceneSequencePlayer.OnFinished` _sequenceplayer (`|CreateDelegate` :!event `OnLSPlayFinished`))))

(event `OnLSPlayFinished`
  (`self.OnLevelSequencePlayEnded`)
  (if (`self.EnableFadeIn`)
    (`self.OnFadeInStart`)
    (bind _createdwidget (`self.FadeIn_Implementation` (stale `self.ReceiveActorBeginOverlap` `_asプレイヤーコントローラー`)))
    (`KismetSystemLibrary.Delay` (`self.FadeInTime`))
    (`self.OnFadeInEnd`)
    (`Widget.RemoveFromParent` _createdwidget)
    (`KismetSystemLibrary.CollectGarbage`))
  (if (`self.bAutoDestroy`)
    (`self.K2_DestroyActor`)))

(fn `FadeIn_Implementation`
  (params (PlayerController :type "PlayerController Object Reference (by ref)"))
  (returns (CreatedWidget :type "UserWidget Object Reference"))
  (bind _returnvalue (`|CreateWidget` "/Game/TestResources/Yamauchi/WBP_Fade.WBP_Fade_C" PlayerController))
  (`UserWidget.AddToViewport` _returnvalue 0)
  (`/Game/TestResources/Yamauchi/WBP_Fade.FadeInEvent_Event` _returnvalue)
  (return _returnvalue))

(fn `FadeOut_Implementation`
  (params (PlayerController :type "PlayerController Object Reference"))
  (returns (CreatedWidget :type "UserWidget Object Reference"))
  (bind _returnvalue (`|CreateWidget` "/Game/TestResources/Yamauchi/WBP_Fade.WBP_Fade_C" PlayerController))
  (`UserWidget.AddToViewport` _returnvalue 0)
  (`/Game/TestResources/Yamauchi/WBP_Fade.FadeOutEvent_Event` _returnvalue)
  (return _returnvalue))

(fn `UserConstructionScript`)