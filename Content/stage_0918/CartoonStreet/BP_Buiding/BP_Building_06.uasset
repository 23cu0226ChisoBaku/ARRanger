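; Cartoon street building actor that varies which of its windows appear lit.
; When the Light flag is set, the construction script picks one of two fixed window layouts at random, swapping glass material slots between two emissive variants and unlit glass.
; The main building mesh gets emissive glass in both layouts.
; The roll is unseeded, and the event graph holds no active logic.
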(fn `UserConstructionScript`
  (bind _sm_building_07_window_02 (`self.SM_Building_07_Window_02`))
  (bind _sm_building_07_window_04 (`self.SM_Building_07_Window_04`))
  (bind _sm_building_07 (`self.SM_Building_07`))
  (if (`self.Light`)
    (if (>= (`KismetMathLibrary.RandomFloatInRange` 0.0 1.0) 0.5)
      ;[1 1 1] Light1
      (`PrimitiveComponent.SetMaterial` _sm_building_07_window_02 1 "/Game/stage_0918/CartoonStreet/Materials/Glass/MI_Glass_Emissive.MI_Glass_Emissive")
      (`PrimitiveComponent.SetMaterial` (`self.SM_Building_07_Window_05`) 1 "/Game/stage_0918/CartoonStreet/Materials/Glass/MI_Glass_Emissive.MI_Glass_Emissive")
      ;[1 1 1] Light2
      (`PrimitiveComponent.SetMaterial` (`self.SM_Building_07_Window_03`) 1 "/Game/stage_0918/CartoonStreet/Materials/Glass/MI_Glass_Emissive1.MI_Glass_Emissive1")
      (`PrimitiveComponent.SetMaterial` (`self.SM_Building_07_Window_01`) 1 "/Game/stage_0918/CartoonStreet/Materials/Glass/MI_Glass_Emissive1.MI_Glass_Emissive1")
      ;[1 1 1] NoLight
      (`PrimitiveComponent.SetMaterial` _sm_building_07_window_04 1 "/Game/stage_0918/CartoonStreet/Materials/Glass/MI_Glass_01.MI_Glass_01")
      (`PrimitiveComponent.SetMaterial` _sm_building_07 1 "/Game/stage_0918/CartoonStreet/Materials/Glass/MI_Glass_Emissive.MI_Glass_Emissive")
      (else
        ;[1 1 1] Light1
        (`PrimitiveComponent.SetMaterial` _sm_building_07_window_04 1 "/Game/stage_0918/CartoonStreet/Materials/Glass/MI_Glass_Emissive.MI_Glass_Emissive")
        (`PrimitiveComponent.SetMaterial` (`self.SM_Building_07_Window_05`) 1 "/Game/stage_0918/CartoonStreet/Materials/Glass/MI_Glass_Emissive.MI_Glass_Emissive")
        ;[1 1 1] Light2
        (`PrimitiveComponent.SetMaterial` (`self.SM_Building_07_Window_01`) 1 "/Game/stage_0918/CartoonStreet/Materials/Glass/MI_Glass_Emissive1.MI_Glass_Emissive1")
        ;[1 1 1] NoLight
        (`PrimitiveComponent.SetMaterial` _sm_building_07_window_02 1 "/Game/stage_0918/CartoonStreet/Materials/Glass/MI_Glass_01.MI_Glass_01")
        (`PrimitiveComponent.SetMaterial` (`self.SM_Building_07_Window_03`) 1 "/Game/stage_0918/CartoonStreet/Materials/Glass/MI_Glass_01.MI_Glass_01")
        (`PrimitiveComponent.SetMaterial` _sm_building_07 1 "/Game/stage_0918/CartoonStreet/Materials/Glass/MI_Glass_Emissive.MI_Glass_Emissive")))))