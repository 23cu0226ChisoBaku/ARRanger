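; BP_Building_03_A is a cartoon street building for a level that can show randomly lit windows.
; When the Light flag is set, its construction script randomly picks one of two patterns, assigning each window mesh one of two emissive glass materials or a dark glass material.
; In both patterns one glass slot on the main building mesh becomes emissive.
; The event graph holds only disabled placeholder events.
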(fn `UserConstructionScript`
  (bind _sm_building_03_window_01 (`self.SM_Building_03_Window_01`))
  (bind _sm_building_03 (`self.SM_Building_03`))
  (if (`self.Light`)
    (if (>= (`KismetMathLibrary.RandomFloatInRange` 0.0 1.0) 0.5)
      ;[1 1 1] Light1
      (`PrimitiveComponent.SetMaterial` _sm_building_03_window_01 1 "/Game/Level/stage_0922/CartoonStreet/Materials/Glass/MI_Glass_Emissive.MI_Glass_Emissive")
      ;[1 1 1] Light2
      (`PrimitiveComponent.SetMaterial` (`self.SM_Window_02`) 1 "/Game/Level/stage_0922/CartoonStreet/Materials/Glass/MI_Glass_Emissive1.MI_Glass_Emissive1")
      (`PrimitiveComponent.SetMaterial` (`self.SM_Building_03_Window_03`) 1 "/Game/Level/stage_0922/CartoonStreet/Materials/Glass/MI_Glass_Emissive1.MI_Glass_Emissive1")
      ;[1 1 1] NoLight
      (`PrimitiveComponent.SetMaterial` (`self.SM_Window_03`) 1 "/Game/Level/stage_0922/CartoonStreet/Materials/Glass/MI_Glass_01.MI_Glass_01")
      (`PrimitiveComponent.SetMaterial` (`self.SM_Building_03_Window_04`) 1 "/Game/Level/stage_0922/CartoonStreet/Materials/Glass/MI_Glass_01.MI_Glass_01")
      (`PrimitiveComponent.SetMaterial` (`self.SM_Building_03_Window_02`) 1 "/Game/Level/stage_0922/CartoonStreet/Materials/Glass/MI_Glass_01.MI_Glass_01")
      (`PrimitiveComponent.SetMaterial` _sm_building_03 5 "/Game/Level/stage_0922/CartoonStreet/Materials/Glass/MI_Glass_Emissive.MI_Glass_Emissive")
      (else
        ;[1 1 1] Light1
        (`PrimitiveComponent.SetMaterial` (`self.SM_Window_03`) 1 "/Game/Level/stage_0922/CartoonStreet/Materials/Glass/MI_Glass_Emissive.MI_Glass_Emissive")
        (`PrimitiveComponent.SetMaterial` (`self.SM_Building_03_Window_03`) 1 "/Game/Level/stage_0922/CartoonStreet/Materials/Glass/MI_Glass_Emissive.MI_Glass_Emissive")
        (`PrimitiveComponent.SetMaterial` (`self.SM_Building_03_Window_04`) 1 "/Game/Level/stage_0922/CartoonStreet/Materials/Glass/MI_Glass_Emissive.MI_Glass_Emissive")
        ;[1 1 1] Light2
        (`PrimitiveComponent.SetMaterial` _sm_building_03_window_01 1 "/Game/Level/stage_0922/CartoonStreet/Materials/Glass/MI_Glass_Emissive1.MI_Glass_Emissive1")
        (`PrimitiveComponent.SetMaterial` (`self.SM_Building_03_Window_02`) 1 "/Game/Level/stage_0922/CartoonStreet/Materials/Glass/MI_Glass_Emissive1.MI_Glass_Emissive1")
        ;[1 1 1] NoLight
        (`PrimitiveComponent.SetMaterial` (`self.SM_Window_02`) 1 "/Game/Level/stage_0922/CartoonStreet/Materials/Glass/MI_Glass_01.MI_Glass_01")
        (`PrimitiveComponent.SetMaterial` _sm_building_03 5 "/Game/Level/stage_0922/CartoonStreet/Materials/Glass/MI_Glass_Emissive.MI_Glass_Emissive")))))