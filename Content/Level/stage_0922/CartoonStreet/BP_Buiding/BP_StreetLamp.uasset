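; BP_StreetLamp is a street lamp actor for the CartoonStreet level, configured in the Construction Script, with no active event logic.
; When Light is set, it toggles the RectLight's visibility, applies the Intensity and Shadow variables, and assigns an emissive material to the lamp mesh.
; Visibility is flipped rather than set explicitly, so the result depends on the component's default.
; A volumetric scattering node is left disconnected.
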(fn `UserConstructionScript`
  (bind _rectlight (`self.RectLight`))
  (if (`self.Light`)
    (`SceneComponent.ToggleVisibility` _rectlight true)
    (`LightComponent.SetIntensity` _rectlight (`self.Intensity`))
    (`LightComponentBase.SetCastShadows` _rectlight (`self.Shadow`))
    (`PrimitiveComponent.SetMaterial` (`self.SM_StreeLamp_01`) 3 "/Game/Level/stage_0922/CartoonStreet/Materials/Glass/MI_Light_Emissive.MI_Light_Emissive")))