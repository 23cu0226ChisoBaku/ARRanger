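; Default charge-attack gameplay ability that reports press-and-hold input to the avatar pawn's ARRangerPlayerController.
; On press, it registers a hold with input-block and ignore tags, then stores the returned handle and start time.
; On release, it ends that hold by passing the handle and elapsed held time to the controller.
; The graph implements only these input events, leaving activation and end events as disabled placeholders.
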(event `self.K2_InputPressed`
  (bind `_asポーン` (cast `Pawn` (`self.GetAvatarActorFromActorInfo`)))
  (bind _asarranger_player_controller (cast `ARRangerPlayerController` (`Pawn.GetController` `_asポーン`)))
  (bind _returnvalue (`ARRangerPlayerController.OnGameplayAbilityActivated_Hold` _asarranger_player_controller (`self.bBlockInputWhenActive`) (`self.InputBlockIgnoreTagContainer`)))
  (set `self.HoldHandle` _returnvalue)
  (set `self.HeldTimeCount` (`GameplayStatics.GetTimeSeconds`)))

(event `self.K2_InputReleased`
  (cast `Pawn` (`self.GetAvatarActorFromActorInfo`))
  (bind _asarranger_player_controller (cast `ARRangerPlayerController` (`Pawn.GetController` (stale `self.K2_InputPressed` `_asポーン`))))
  (`ARRangerPlayerController.OnGameplayAbilityEnded_Hold` _asarranger_player_controller (`self.HoldHandle`) (- (`GameplayStatics.GetTimeSeconds`) (`self.HeldTimeCount`))))