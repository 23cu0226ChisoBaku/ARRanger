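; Gameplay ability for the middle boss enemy's jump attack, handling what happens when the attack's animation finishes.
; On activation it binds to the mesh AnimInstance's montage-ended event; the graph itself plays no montage.
; The finish handler calls the boss's OnAttackFinished and resets its rotation to yaw only.
; OnEndAbility is empty and the unbind logic is unconnected, so this graph never removes the binding.
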(event `self.K2_ActivateAbility`
  (bind _asenemy_middle_boss (cast `Enemy_MiddleBoss` (`self.GetAvatarActorFromActorInfo`)))
  (bind _returnvalue (`SkeletalMeshComponent.GetAnimInstance` (`Character.Mesh` _asenemy_middle_boss)))
  (if (`KismetSystemLibrary.IsValid` _returnvalue)
    (add `AnimInstance.OnMontageEnded` _returnvalue (`|CreateDelegate` :!event `OnMiddleBossJumpAttackFinishedEvent`))))

(event `OnMiddleBossJumpAttackFinishedEvent`
  (params (Montage :type "AnimMontage Object Reference") (bInterrupted :type Boolean))
  (bind _asenemy_middle_boss (cast `Enemy_MiddleBoss` (`self.GetAvatarActorFromActorInfo`)))
  (`Enemy_MiddleBoss.K2_OnAttackFinished` _asenemy_middle_boss)
  (bind (_returnvalue_roll _returnvalue_pitch _returnvalue_yaw) (`KismetMathLibrary.BreakRotator` (`Actor.K2_GetActorRotation` _asenemy_middle_boss)))
  (`Actor.K2_SetActorRotation` _asenemy_middle_boss (`KismetMathLibrary.MakeRotator` 0.0 0.0 _returnvalue_yaw) false))