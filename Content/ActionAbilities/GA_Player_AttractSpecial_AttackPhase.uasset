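; Player gameplay ability for the attack phase of the Attract special.
; On activation it calls PerformSpecialAttract on the avatar's AttractSpecialAttackComponent, which holds the attack logic.
; When the ability ends, cancelled or not, it activates the end-phase ability by the Ability.Special.AttractEndPhase tag, chaining the special's phases.
; The graph never ends the ability itself.
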(event `self.K2_ActivateAbility`
  (bind _returnvalue (`Actor.GetComponentByClass` (`self.GetAvatarActorFromActorInfo`) "/Script/ARRanger.AttractSpecialAttackComponent"))
  (`parent.K2_ActivateAbility`)
  (if (`KismetSystemLibrary.IsValid` _returnvalue)
    (`AttractSpecialAttackComponent.PerformSpecialAttract` _returnvalue)))

(event `self.K2_OnEndAbility`
  (params (bWasCancelled :type Boolean))
  (bind _returnvalue (`self.GetAbilitySystemComponentFromActorInfo`))
  (`parent.K2_OnEndAbility` bWasCancelled)
  (if (`KismetSystemLibrary.IsValid` _returnvalue)
    (`AbilitySystemComponent.TryActivateAbilitiesByTag` _returnvalue (`BlueprintGameplayTagLibrary.MakeLiteralGameplayTagContainer` (struct :`GameplayTags` (struct :`(TagName` "Ability.Special.AttractEndPhase")))) true)))