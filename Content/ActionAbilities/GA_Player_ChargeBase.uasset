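; GA_Player_ChargeBase is a gameplay ability, apparently a base for player hold-to-charge abilities, that registers holds with the Ranger player controller.
; On activation it calls the parent, then notifies the controller with input-block and ignore tags, storing the returned hold handle.
; On end it returns that handle and the held time to the controller before calling the parent end logic.
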(event `self.K2_ActivateAbility`
  (`parent.K2_ActivateAbility`)
  (bind `_asポーン` (cast `Pawn` (`self.GetAvatarActorFromActorInfo`)))
  (bind _asarranger_player_controller (cast `ARRangerPlayerController` (`Pawn.GetController` `_asポーン`)))
  (bind _returnvalue (`ARRangerPlayerController.OnGameplayAbilityActivated_Hold` _asarranger_player_controller (`self.bBlockInput`) (`self.InputBlockIgnoreTags`)))
  (set `self.HoldHandle` _returnvalue))

(event `self.K2_OnEndAbility`
  (params (bWasCancelled :type Boolean))
  (bind `_asポーン` (cast `Pawn` (`self.GetAvatarActorFromActorInfo`)))
  (bind _asarranger_player_controller (cast `ARRangerPlayerController` (`Pawn.GetController` `_asポーン`)))
  (`ARRangerPlayerController.OnGameplayAbilityEnded_Hold` _asarranger_player_controller (`self.HoldHandle`) (`self.GetHeldTime`))
  (`parent.K2_OnEndAbility` bWasCancelled))