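; Gameplay ability for the start phase of the player's special attract attack.
; On activation it calls StartSpecialAttract on the avatar's AttractSpecialAttackComponent, if that component is valid.
; When the ability ends, cancelled or not, it activates the Ability.Special.AttractAttackPhase ability by tag, chaining into the attack phase.
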(event `self.K2_ActivateAbility`
  (bind _returnvalue (`Actor.GetComponentByClass` (`self.GetAvatarActorFromActorInfo`) "/Script/ARRanger.AttractSpecialAttackComponent"))
  (`parent.K2_ActivateAbility`)
  (if (`KismetSystemLibrary.IsValid` _returnvalue)
    (`AttractSpecialAttackComponent.StartSpecialAttract` _returnvalue)))

(event `self.K2_OnEndAbility`
  (params (bWasCancelled :type Boolean))
  (`parent.K2_OnEndAbility` bWasCancelled)
  (`AbilitySystemComponent.TryActivateAbilitiesByTag` (`self.GetAbilitySystemComponentFromActorInfo`) (`BlueprintGameplayTagLibrary.MakeLiteralGameplayTagContainer` (struct :`GameplayTags` (struct :`(TagName` "Ability.Special.AttractAttackPhase")))) true))