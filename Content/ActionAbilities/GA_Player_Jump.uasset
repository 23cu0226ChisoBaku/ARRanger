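; Player jump gameplay ability that reports its activation and end to the ARRanger player controller.
; On activation it finds the controller through the avatar pawn and passes it the InputState.OnAir tag.
; On end it forwards the cancelled flag to the same controller class, if the controller is valid.
; The graph itself applies no jump movement and never calls EndAbility.
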(event `self.K2_ActivateAbility`
  (bind `_asポーン` (cast `Pawn` (`self.GetAvatarActorFromActorInfo`)))
  (bind _asarranger_player_controller (cast `ARRangerPlayerController` (`Pawn.GetController` `_asポーン`)))
  (`ARRangerPlayerController.OnGameplayAbilityActivate` _asarranger_player_controller (`BlueprintGameplayTagLibrary.MakeLiteralGameplayTag` (struct :`TagName` "InputState.OnAir"))))

(event `self.K2_OnEndAbility`
  (params (bWasCancelled :type Boolean))
  (bind _returnvalue (`self.GetController`))
  (if (`KismetSystemLibrary.IsValid` _returnvalue)
    (bind _asarranger_player_controller (cast `ARRangerPlayerController` _returnvalue))
    (`ARRangerPlayerController.OnGameplayAbilityEnd` _asarranger_player_controller bWasCancelled)))