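; Short-lived hit effect actor that shows a WBP_Bang widget through its widget component.
; On BeginPlay it randomly nudges the position and angle of the widget's SizeBox56, then sets a raised, enlarged render transform, which appears to overwrite that random angle.
; Tick counts DeadTimeInterval down by delta time and destroys the actor once it runs out.
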(event `self.ReceiveBeginPlay`
  (bind _aswbp_bang (cast `/Game/TestResources/Mai/PhysicsTest/WBP_Bang` (`WidgetComponent.GetUserWidgetObject` (`self.Widget`))))
  (bind _sizebox_56 (`/Game/TestResources/Mai/PhysicsTest/WBP_Bang.SizeBox_56` _aswbp_bang))
  (bind `_asキャンバスパネルスロット` (cast `CanvasPanelSlot` (`Widget.Slot` _sizebox_56)))
  (`CanvasPanelSlot.SetPosition` `_asキャンバスパネルスロット` (`KismetMathLibrary.MakeVector2D` (`KismetMathLibrary.RandomFloatInRange` -1.0 1.0) (`KismetMathLibrary.RandomFloatInRange` -1.0 1.0)))
  (`Widget.SetRenderTransformAngle` _sizebox_56 (`KismetMathLibrary.RandomFloatInRange` -15.0 15.0))
  (`Widget.SetRenderTransform` _sizebox_56 (make `WidgetTransform` (0.0 -10.0) (1.5 1.5))))

(event `self.ReceiveTick`
  (params (DeltaSeconds :type "Float (single-precision)"))
  (set `self.DeadTimeInterval` (- (`self.DeadTimeInterval`) DeltaSeconds))
  (if (<= (`self.DeadTimeInterval`) 0.0)
    (`self.K2_DestroyActor`)))

(fn `UserConstructionScript`)