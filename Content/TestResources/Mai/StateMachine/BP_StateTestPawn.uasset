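; BP_StateTestPawn is a test pawn that exercises a gameplay-tag-driven state machine.
; On BeginPlay it registers three state definitions, sets the entry state by tag and starts ticking the machine.
; Holding key 1 or key 2 switches to a second or third tagged state, and releasing either key returns to the entry tag's state.
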(event `self.ReceiveBeginPlay`
  (`MStateMachineComponent.AddNewState` "/Game/TestResources/Mai/StateMachine/BP_StateDef_1.BP_StateDef_1_C")
  (`MStateMachineComponent.AddNewState` "/Game/TestResources/Mai/StateMachine/BP_StateDef_2.BP_StateDef_2_C")
  (`MStateMachineComponent.AddNewState` "/Game/TestResources/Mai/StateMachine/BP_StateDef_3.BP_StateDef_3_C")
  (`MStateMachineComponent.SetEntryState` (`BlueprintGameplayTagLibrary.MakeLiteralGameplayTag` (struct :`TagName` "Test.StateTree.Tag")))
  (`MStateMachineComponent.StartTickState`))

(event `Key|One`
  (params (Key :type "Key Structure"))
  (:`Pressed`
    (`MStateMachineComponent.SwitchNextState` (`BlueprintGameplayTagLibrary.MakeLiteralGameplayTag` (struct :`TagName` "Test.StateTree.Tag2"))))
  (:`Released`
    (`MStateMachineComponent.SwitchNextState` (`BlueprintGameplayTagLibrary.MakeLiteralGameplayTag` (struct :`TagName` "Test.StateTree.Tag")))))

(event `Key|Two`
  (params (Key :type "Key Structure"))
  (:`Pressed`
    (`MStateMachineComponent.SwitchNextState` (`BlueprintGameplayTagLibrary.MakeLiteralGameplayTag` (struct :`TagName` "Test.StateTree.Tag3"))))
  (:`Released`
    (`MStateMachineComponent.SwitchNextState` (`BlueprintGameplayTagLibrary.MakeLiteralGameplayTag` (struct :`TagName` "Test.StateTree.Tag")))))

(fn `UserConstructionScript`)