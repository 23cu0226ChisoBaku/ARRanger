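; BP_GhostTrail is a test Blueprint that, despite its name, holds keyboard and mouse controls for a Gameplay Camera.
; Number keys 1 to 3 set the ActiveCameraRig index.
; The mouse wheel steps a clamped BoomLength and passes it as the X boom offset to the camera rig parameters on the GameplayCamera's initial result.
; Wheel-up also prints a debug string, and the construction script is empty.
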(event `Key|One`
  (params (Key :type "Key Structure"))
  (:`Pressed`
    (set `self.ActiveCameraRig` 0)))

(event `Key|Two`
  (params (Key :type "Key Structure"))
  (:`Pressed`
    (set `self.ActiveCameraRig` 1)))

(event `Key|Three`
  (params (Key :type "Key Structure"))
  (:`Pressed`
    (set `self.ActiveCameraRig` 2)))

(event `Key|MouseScrollUp`
  (params (Key :type "Key Structure"))
  (:`Pressed`
    (set `self.BoomLength` (`KismetMathLibrary.FClamp` (+ (`self.BoomLength`) (`self.BoomZoomStep`)) -1000.0 0.0))
    (`KismetSystemLibrary.PrintString` "Hello")
    (`|SetCameraRigParameters` (`GameplayCameraComponentBase.GetInitialResult` (`self.GameplayCamera`)) (`KismetMathLibrary.MakeVector` (`self.BoomLength`)))))

(event `Key|MouseScrollDown`
  (params (Key :type "Key Structure"))
  (:`Pressed`
    (set `self.BoomLength` (`KismetMathLibrary.FClamp` (- (`self.BoomLength`) (`self.BoomZoomStep`)) -1000.0 0.0))
    (`|SetCameraRigParameters` (`GameplayCameraComponentBase.GetInitialResult` (`self.GameplayCamera`)) (`KismetMathLibrary.MakeVector` (`self.BoomLength`)))))

(fn `UserConstructionScript`)