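; Test actor that animates an outline on its static mesh through a dynamic material instance.
; BeginPlay creates the instance from the mesh's current overlay material.
; Tick accumulates delta time, drives the Outline Width parameter with a scaled absolute cosine for a pulsing effect, and reassigns the instance as the overlay material every frame.
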(event `self.ReceiveBeginPlay`
  (bind _returnvalue (`KismetMaterialLibrary.CreateDynamicMaterialInstance` (`MeshComponent.GetOverlayMaterial` (`self.StaticMesh`))))
  (set `self.NewVar_0` _returnvalue))

(event `self.ReceiveTick`
  (params (DeltaSeconds :type "Float (single-precision)"))
  (bind _output_get (set `self.NewVar` (+ DeltaSeconds (`self.NewVar`))))
  (`MaterialInstanceDynamic.SetScalarParameterValue` (`self.NewVar_0`) "Outline Width" (`KismetMathLibrary.Abs` (* (`KismetMathLibrary.Cos` _output_get) 200.0)))
  (`MeshComponent.SetOverlayMaterial` (`self.StaticMesh`) (`self.NewVar_0`)))

(fn `UserConstructionScript`)