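; Battle event manager Blueprint that links battle field state to the enemy-count display on the player UI.
; On BeginPlay it binds to the start and end of any field battle, alongside events that start and end the enemy-count UI.
; Tick polls the phase's remaining enemy count, debug-prints it and pushes it to the player widget when valid.
; The widget is supplied through a setter event, whose loop over all battle fields is empty.
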(event `self.ReceiveBeginPlay`
  (add `self.OnAnyFieldBattleStart` (`|CreateDelegate` :!event `StartEnemyNumUI`))
  (add `self.OnAnyFieldBattleEnd` (`|CreateDelegate` :!event `EndEnemyNumUI`)))

(event `self.ReceiveTick`
  (params (DeltaSeconds :type "Float (single-precision)"))
  (bind _returnvalue (`self.GetCurrentRemainingEnemiesInPhase`))
  (bind _playeruiwbp (`self.PlayerUIWBP`))
  (`KismetSystemLibrary.PrintString` (`KismetStringLibrary.Conv_IntToString` _returnvalue))
  (`/Engine/EditorBlueprintResources/StandardMacros.IsValid` _playeruiwbp
    (:`Is Valid`
      (`/Game/WBP_PlayerMainUI_KARI.SetRemainingnumber_Event` _playeruiwbp _returnvalue))))

(event `SetPlayerUIWBP_Event`
  (params (playerUIWBP :type "/Game/WBP_PlayerMainUI_KARI Object Reference"))
  (set `self.PlayerUIWBP` playerUIWBP)
  (for _ (`self.GetAllBattleField`)
    _))

(event `StartEnemyNumUI`
  (`/Game/WBP_PlayerMainUI_KARI.StartEnemyNumUI_Event` (`self.PlayerUIWBP`)))

(event `EndEnemyNumUI`
  (`/Game/WBP_PlayerMainUI_KARI.EndEnemyNumUI_Event` (`self.PlayerUIWBP`)))

(fn `UserConstructionScript`)