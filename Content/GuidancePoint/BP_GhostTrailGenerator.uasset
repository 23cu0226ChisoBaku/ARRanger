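; Actor that leaves a ghost trail by spawning short-lived afterimage actors at its own transform.
; While not hidden, Tick accumulates time and calls GenerateGhostTrail each time the interval elapses.
; Each spawned BP_GhostTrailActor gets a lifespan, the configured static mesh and a dynamic M_GhostTrail material carrying the trail color and clamped opacity.
; SetGhostTrailColor changes the color used for subsequently spawned ghosts.
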(event `self.ReceiveTick`
  (params (DeltaSeconds :type "Float (single-precision)"))
  (if (not (`self.bHidden`))
    (`self.Evaluate Ghost Trail` DeltaSeconds)))

(fn `Evaluate Ghost Trail`
  (params (DeltaTime :type "Float (double-precision)"))
  (bind _output_get (set `self.GhostTrailGenerateTimeCnt` (+ DeltaTime (`self.GhostTrailGenerateTimeCnt`))))
  (if (>= _output_get (`self.GhostTrailGenerateTimeInterval`))
    (set `self.GhostTrailGenerateTimeCnt` 0.0)
    (`self.Generate Ghost Trail` (`self.GhostTrailOpacity`))))

(fn `Generate Ghost Trail`
  (params (TrailOpacity :type "Float (double-precision)"))
  (bind _returnvalue (`|SpawnActorFromClass` "/Game/GuidancePoint/BP_GhostTrailActor.BP_GhostTrailActor_C" (`self.GetTransform`) "AlwaysSpawn" "MultiplyWithRoot" null null))
  (`self.SetLifeSpan` _returnvalue (`self.GhostTrailLifeTime`))
  (bind _staticmeshcomponent (`StaticMeshActor.StaticMeshComponent` _returnvalue))
  (`StaticMeshComponent.SetStaticMesh` _staticmeshcomponent (`self.GhostTrailStaticMesh`))
  (bind _returnvalue_2 (`PrimitiveComponent.CreateDynamicMaterialInstance` _staticmeshcomponent 0 "/Game/GuidancePoint/M_GhostTrail.M_GhostTrail" "MID_GhostTrail"))
  (`MaterialInstanceDynamic.SetVectorParameterValue` _returnvalue_2 "TrailColor" (`self.GhostTrailColor`))
  (`MaterialInstanceDynamic.SetScalarParameterValue` _returnvalue_2 "Opacity" (`KismetMathLibrary.FClamp` TrailOpacity))
  (`PrimitiveComponent.SetMaterial` _staticmeshcomponent 0 _returnvalue_2))

(fn `Set Ghost Trail Color`
  (params (`In Color` :type "LinearColor Structure"))
  (set `self.GhostTrailColor` `In Color`))

(fn `UserConstructionScript`)