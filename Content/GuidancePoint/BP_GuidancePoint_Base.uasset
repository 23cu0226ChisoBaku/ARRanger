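; Base Blueprint for a guidance point actor that shows attraction or repulsion by color and vanishes when terminated.
; Attraction and repulsion change events apply a new dynamic material instance with the matching color, while activation toggles mesh visibility.
; Termination disables collision overlap events, counts up to an interval, then spawns a Niagara vanish effect tinted with the mesh's current base color and destroys the actor.
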(event `self.K2_OnTerminationStarted`
  (set `PrimitiveComponent.bGenerateOverlapEvents` false (`self.GuidancePointCollision`)))

(event `self.K2_OnTerminationEventUpdated`
  (params (DeltaTime :type "Float (single-precision)"))
  (bind _output_get (set `self.TerminateTimeCount` (+ DeltaTime (`self.TerminateTimeCount`))))
  (if (>= _output_get (`self.TerminateTimeInterval`))
    (`self.OnTerminationEnded`)))

(event `self.K2_OnTerminationEnded`
  (bind _pointmesh (`self.PointMesh`))
  (bind _returnvalue (`NiagaraFunctionLibrary.SpawnSystemAtLocation` "/Game/Effects/Particle/NS_Particle_Vanish.NS_Particle_Vanish" (`SceneComponent.K2_GetComponentLocation` (`self.PointMesh`))))
  (bind _returnvalue_2 (`PrimitiveComponent.CreateDynamicMaterialInstance` _pointmesh 0 (`PrimitiveComponent.GetMaterial` _pointmesh 0) "MID_Temp"))
  (bind _returnvalue_3 (`MaterialInstanceDynamic.K2_GetVectorParameterValue` _returnvalue_2 (`self.M_BaseColorName`)))
  (`NiagaraComponent.SetVariableLinearColor` _returnvalue "Color" _returnvalue_3)
  (`self.K2_DestroyActor`))

(event `self.K2_OnActivationSet`
  (params (bActive :type Boolean))
  (`SceneComponent.SetHiddenInGame` (`self.PointMesh`) (not bActive) false)
  (if bActive
    _))

(event `self.K2_OnAttractionChanged`
  (`self.BPF_OnAttractionChanged`))

(event `self.K2_OnRepulsionChanged`
  (`self.BPF_OnRepulsionChanged`))

(fn `BPF_ChangeMaterial`
  (params (BaseColor :type "LinearColor Structure") (EmissiveColor :type "LinearColor Structure") (Opacity :type "Float (double-precision)"))
  (bind _returnvalue (`KismetMaterialLibrary.CreateDynamicMaterialInstance` "/Game/GuidancePoint/M_GuidancePoint.M_GuidancePoint" "MID_AttractionPoint" "Transient"))
  (`MaterialInstanceDynamic.SetVectorParameterValue` _returnvalue (`self.M_BaseColorName`) BaseColor)
  (`MaterialInstanceDynamic.SetVectorParameterValue` _returnvalue (`self.M_EmissiveColorName`) EmissiveColor)
  (`MaterialInstanceDynamic.SetScalarParameterValue` _returnvalue (`self.M_OpacityName`) Opacity)
  (`MaterialInstanceDynamic.SetScalarParameterValue` _returnvalue (`self.M_EmissiveStrengthName`) (`self.EmissiveLightStrength`))
  (`PrimitiveComponent.SetMaterial` (`self.PointMesh`) 0 _returnvalue))

(fn `BPF_OnAttractionChanged`
  (bind _attractiontypecolor (`self.AttractionTypeColor`))
  (`self.BPF_ChangeMaterial` _attractiontypecolor _attractiontypecolor 1.0))

(fn `BPF_OnRepulsionChanged`
  (bind _repulsiontypecolor (`self.RepulsionTypeColor`))
  (`self.BPF_ChangeMaterial` _repulsiontypecolor _repulsiontypecolor 1.0))

(fn `UserConstructionScript`)