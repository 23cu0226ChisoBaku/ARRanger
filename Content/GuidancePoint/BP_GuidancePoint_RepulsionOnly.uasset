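; Guidance point variant that is active only in the repulsion state, as a child Blueprint overriding the parent's polarity-change functions.
; Switching to attraction skips the parent logic, fades the material to a dim, nearly transparent attraction color, and disables collision overlap events and the ghost trail.
; Switching to repulsion runs the parent behavior, then re-enables overlap events and ghost trail generation.
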(fn `BPF_OnAttractionChanged`
  (`self.BPF_ChangeMaterial` (* (`self.AttractionTypeColor`) 0.3) (struct) 0.05)
  (set `PrimitiveComponent.bGenerateOverlapEvents` false (`self.GuidancePointCollision`))
  (set `/Game/GuidancePoint/BP_GhostTrailGenerator.bCanGenerateGhostTrail` false (`self.GhostTrailActor`)))

(fn `BPF_OnRepulsionChanged`
  (`parent.BPF_OnRepulsionChanged`)
  (set `PrimitiveComponent.bGenerateOverlapEvents` true (`self.GuidancePointCollision`))
  (set `/Game/GuidancePoint/BP_GhostTrailGenerator.bCanGenerateGhostTrail` true (`self.GhostTrailActor`)))

(fn `UserConstructionScript`
  (`parent.UserConstructionScript`))