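; BP_Building_01 is a cartoon street building with window meshes that can appear lit.
; When Light is set, the Construction Script randomly picks one of two lighting patterns, assigning two emissive glass variants to the windows' second material slot.
; One pattern lights all four windows, while the other leaves SMWindow04 untouched.
; The roll repeats whenever construction reruns, and the event graph has no active logic.
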(fn `UserConstructionScript`
  (if (`self.Light`)
    (if (>= (`KismetMathLibrary.RandomFloatInRange` 0.0 1.0) 0.5)
      (`PrimitiveComponent.SetMaterial` (`self.SM_Window_03`) 1 "/Game/stage/CartoonStreet/Materials/Glass/MI_Glass_Emissive.MI_Glass_Emissive")
      (`PrimitiveComponent.SetMaterial` (`self.SM_Window_02`) 1 "/Game/stage/CartoonStreet/Materials/Glass/MI_Glass_Emissive.MI_Glass_Emissive")
      (`PrimitiveComponent.SetMaterial` (`self.SM_Window_04`) 1 "/Game/stage/CartoonStreet/Materials/Glass/MI_Glass_Emissive1.MI_Glass_Emissive1")
      (`PrimitiveComponent.SetMaterial` (`self.SM_Window_01`) 1 "/Game/stage/CartoonStreet/Materials/Glass/MI_Glass_Emissive1.MI_Glass_Emissive1")
      (else
        (`PrimitiveComponent.SetMaterial` (`self.SM_Window_03`) 1 "/Game/stage/CartoonStreet/Materials/Glass/MI_Glass_Emissive.MI_Glass_Emissive")
        (`PrimitiveComponent.SetMaterial` (`self.SM_Window_02`) 1 "/Game/stage/CartoonStreet/Materials/Glass/MI_Glass_Emissive1.MI_Glass_Emissive1")
        (`PrimitiveComponent.SetMaterial` (`self.SM_Window_01`) 1 "/Game/stage/CartoonStreet/Materials/Glass/MI_Glass_Emissive1.MI_Glass_Emissive1")))))